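; Demo actor that visually explains weapon spread in two stepped debug-draw presentations, using the player's camera and selected weapon.
; PlayDesc1 shows a center trace, the spread cone, then looping random traces within it.
; PlayDesc2 redraws stored random cone directions on a timer, while timelines move them to the camera, lengthen them and lerp them into a tighter cone.
; Both sequences advance the same Desc2Seq counter, one step per call.
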(event `self.ReceiveBeginPlay`
  (`self.EnableInput` (`GameplayStatics.GetPlayerController` 0)))

(event `PlayDesc1`
  (bind _pcamera (`self.PCamera`))
  (bind _returnvalue (* (`/Game/Blueprints/Weapons/BP_Weapon.FireSpread` (`self.PSelectedWeapon`)) 3.0))
  (`/Engine/EditorBlueprintResources/StandardMacros.IncrementInt` (`self.Desc2Seq`)
    (:`  `
      (switch `int` (`self.Desc2Seq`)
        (:`1`
          (bind _returnvalue_2 (`GameplayStatics.GetActorOfClass` "/Game/Blueprints/Characters/BP_FPS_PCharacterP3.BP_FPS_PCharacterP3_C"))
          (bind _output_get (set `self.PCharacter` _returnvalue_2))
          (set `self.PCamera` (`/Game/Blueprints/Characters/BP_FPS_PCharacterP3.Camera` _output_get))
          (set `self.PSelectedWeapon` (`/Game/Blueprints/Characters/BP_FPS_PCharacterP3.SelectedWeapon` _output_get))
          (`WidgetLayoutLibrary.RemoveAllWidgets`))
        (:`2`
          (bind (_outhit _returnvalue_3) (`KismetSystemLibrary.LineTraceSingle` :`Start` (`SceneComponent.K2_GetComponentLocation` (`self.PCamera`)) :`End` (+ (`SceneComponent.K2_GetComponentLocation` (`self.PCamera`)) (* (`SceneComponent.GetForwardVector` (`self.PCamera`)) 100000.0)) :`TraceChannel` "TraceTypeQuery1" :`DrawDebugType` "ForDuration" :`TraceColor` (struct :`R` 0.720833 :`B` 0.010048 :`A` 1.0) :`DrawTime` 25.0))
          (if _returnvalue_3
            _))
        (:`3`
          (`KismetSystemLibrary.DrawDebugConeInDegrees` (`SceneComponent.K2_GetComponentLocation` _pcamera) (`SceneComponent.GetForwardVector` _pcamera) 100000.0 _returnvalue _returnvalue 16 (struct :`G` 1.0 :`B` 0.757329 :`A` 1.0) 50.0 0.4))
        (:`4`
          (`KismetSystemLibrary.K2_SetTimerDelegate` (delegate `RandomLineTraceByConeLoop`) 0.3 true))))))

(event `RandomLineTraceByConeLoop`
  (bind (_outhit _returnvalue) (`KismetSystemLibrary.LineTraceSingle` :`Start` (`SceneComponent.K2_GetComponentLocation` (`self.PCamera`)) :`End` (+ (`SceneComponent.K2_GetComponentLocation` (`self.PCamera`)) (* (`KismetMathLibrary.RandomUnitVectorInConeInDegrees` (`SceneComponent.GetForwardVector` (`self.PCamera`)) (`KismetMathLibrary.RandomFloatInRange` 0.0 (* (`/Game/Blueprints/Weapons/BP_Weapon.FireSpread` (`self.PSelectedWeapon`)) 3.0))) 100000.0)) :`TraceChannel` "TraceTypeQuery1" :`DrawDebugType` "ForDuration" :`TraceColor` (struct :`R` 0.720833 :`B` 0.010048 :`A` 1.0) :`DrawTime` 25.0))
  (if _returnvalue
    _))

(event `PlayDesc2`
  (`/Engine/EditorBlueprintResources/StandardMacros.IncrementInt` (`self.Desc2Seq`)
    (:`  `
      (switch `int` (`self.Desc2Seq`)
        (:`1`
          (bind _returnvalue (`GameplayStatics.GetActorOfClass` "/Game/Blueprints/Characters/BP_FPS_PCharacterP3.BP_FPS_PCharacterP3_C"))
          (bind _output_get (set `self.PCharacter` _returnvalue))
          (set `self.PCamera` (`/Game/Blueprints/Characters/BP_FPS_PCharacterP3.Camera` _output_get))
          (set `self.PSelectedWeapon` (`/Game/Blueprints/Characters/BP_FPS_PCharacterP3.SelectedWeapon` _output_get))
          (`WidgetLayoutLibrary.RemoveAllWidgets`))
        (:`2`
          (`KismetSystemLibrary.K2_SetTimerDelegate` (delegate `DrawLooop`) 0.05 true)
          (`KismetArrayLibrary.Array_Clear` (`self.RandomDirectionArray`))
          (for _ (range 13)
            (`KismetArrayLibrary.Array_Add` (`self.RandomDirectionArray`) (`KismetMathLibrary.RandomUnitVectorInConeInDegrees` (`SceneComponent.GetForwardVector` (`self.PCamera`)) (* (`KismetMathLibrary.RandomFloatInRange` 0.0 (+ (`/Game/Blueprints/Characters/BP_FPS_PCharacterP3.CurrentSpreadFactor` (`self.PCharacter`)) (`/Game/Blueprints/Weapons/BP_Weapon.FireSpread` (`self.PSelectedWeapon`)))) 24.0)))))
        (:`3`
          (set `self.TempStartLoc` (`self.K2_GetActorLocation`))
          (bind (_direction _alpha) (`Timeline|MoveToCamTimeline` :!via `PlayFromStart`)
            (:`Update`
              (`self.K2_SetActorLocation` (`KismetMathLibrary.VLerp` (`self.TempStartLoc`) (`SceneComponent.K2_GetComponentLocation` (`/Game/Blueprints/Characters/BP_FPS_PCharacterP3.Camera` (`self.PCharacter`))) _alpha)))))
        (:`4`
          (bind (_direction_2 _length) (`Timeline|LineLengthTimeline` :!via `PlayFromStart`)
            (:`Update`
              (set `self.LineLength` (`KismetMathLibrary.Lerp` 100.0 500.0 _length)))))
        (:`5`
          (set `self.DrawEndLoc` true))
        (:`6`
          (set `self.StartRandomDirectionArray` (`self.RandomDirectionArray`))
          (`KismetArrayLibrary.Array_Clear` (`self.EndRandomDirectionArray`))
          (for _ (range 13)
            (`KismetArrayLibrary.Array_Add` (`self.EndRandomDirectionArray`) (`KismetMathLibrary.RandomUnitVectorInConeInDegrees` (`SceneComponent.GetForwardVector` (`self.PCamera`)) (* (`KismetMathLibrary.RandomFloatInRange` 0.0 (+ (`/Game/Blueprints/Characters/BP_FPS_PCharacterP3.CurrentSpreadFactor` (`self.PCharacter`)) (`/Game/Blueprints/Weapons/BP_Weapon.FireSpread` (`self.PSelectedWeapon`)))) 1.0))))
          (bind (_direction_3 _length_2) (`Timeline|VectorLerpTimeline` :!via `PlayFromStart`)
            (:`Update`
              (set `self.LineLength` (`KismetMathLibrary.Lerp` 500.0 11000.0 _length_2))
              (for _index (range 13)
                (`KismetArrayLibrary.Array_Set` (`self.RandomDirectionArray`) _index (`KismetMathLibrary.VLerp` (`|GetArrayItem` (`self.StartRandomDirectionArray`) _index) (`|GetArrayItem` (`self.EndRandomDirectionArray`) _index) _length_2))))))))))

(event `DrawLooop`
  (`|ExecutionSequence`
    (:`then_0`
      (for _index (range 13)
        (set `self.RandomDir` (`|GetArrayItem` (`self.RandomDirectionArray`) _index))
        (`KismetSystemLibrary.DrawDebugArrow` (`self.K2_GetActorLocation`) (+ (`self.K2_GetActorLocation`) (* (`self.RandomDir`) (`self.LineLength`))) 1.2 (struct :`R` 1.0 :`G` 0.287456 :`A` 1.0) (`self.DrawDuraction`) 0.5)))
    (:`then_1`
      (for _index_2 (range 13)
        (set `self.RandomDir` (`|GetArrayItem` (`self.RandomDirectionArray`) _index_2))
        (if (`self.DrawEndLoc`)
          (`KismetSystemLibrary.DrawDebugSphere` (+ (`self.K2_GetActorLocation`) (* (`self.RandomDir`) (`self.LineLength`))) 4.0 12 (struct :`G` 1.0 :`B` 0.074223 :`A` 1.0) (`self.DrawDuraction`) 2.0))))))

(fn `UserConstructionScript`)