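; BP_Ammo is an ammo pickup Blueprint that carries a widget component for showing a pickup prompt.
; On BeginPlay it casts that widget to Widget_PickupIndicator and fills its text from the PickupText variable.
; The ShowPickup event shows or hides the widget component based on its visibility flag, and the file contains no collection or ammo-granting logic.
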(event `self.ReceiveBeginPlay`
  (bind _aswidget_pickup_indicator (cast `/Game/Blueprints/Widgets/Widget_PickupIndicator` (`WidgetComponent.GetWidget` (`self.Widget`))))
  (`TextBlock.SetText` (`/Game/Blueprints/Widgets/Widget_PickupIndicator.Text_Pickup` _aswidget_pickup_indicator) (`self.PickupText`)))

(event `ShowPickup`
  (params (InVisible :type Boolean))
  (if InVisible
    (`SceneComponent.SetVisibility` (`self.Widget`) true false)
    (else
      (`SceneComponent.SetVisibility` (`self.Widget`) false false))))

(fn `UserConstructionScript`)