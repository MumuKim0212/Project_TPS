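; Actor with a W_ModeCheck widget that toggles character and shooting practice targets in the level.
; Each click event flips its checkbox, then spawns three targets when checked or destroys all of that class when unchecked.
; Spawning retries random points inside a tagged box's bounds until an overlap test finds free space or attempts run out.
; Character targets use a fixed height and capsule test; shooting targets use a box test.
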(event `Click_CharacterTarget`
  (bind _asw_mode_check (cast `/Game/Blueprints/Widgets/W_ModeCheck` (`WidgetComponent.GetWidget` (`self.Widget`))))
  (bind _checkbox_charactertarget (`/Game/Blueprints/Widgets/W_ModeCheck.CheckBox_CharacterTarget` _asw_mode_check))
  (bind _returnvalue (not (`CheckBox.IsChecked` _checkbox_charactertarget)))
  (`CheckBox.SetIsChecked` _checkbox_charactertarget _returnvalue)
  (if _returnvalue
    (bind _outactors (`GameplayStatics.GetAllActorsOfClass` "/Game/Blueprints/Targets/BP_FPS_EnemyTarget.BP_FPS_EnemyTarget_C"))
    (for _array_element _outactors
      (`self.K2_DestroyActor` _array_element))
    (else
      (`self.SpawnCharacterTarget`)
      (`self.SpawnCharacterTarget`)
      (`self.SpawnCharacterTarget`))))

(event `Click_ShootingTarget`
  (bind _asw_mode_check (cast `/Game/Blueprints/Widgets/W_ModeCheck` (`WidgetComponent.GetWidget` (`self.Widget`))))
  (bind _checkbox_shootingtarget (`/Game/Blueprints/Widgets/W_ModeCheck.CheckBox_ShootingTarget` _asw_mode_check))
  (bind _returnvalue (not (`CheckBox.IsChecked` _checkbox_shootingtarget)))
  (`CheckBox.SetIsChecked` _checkbox_shootingtarget _returnvalue)
  (if _returnvalue
    (bind _outactors (`GameplayStatics.GetAllActorsOfClass` "/Game/Blueprints/Targets/BP_ShootingTarget.BP_ShootingTarget_C"))
    (for _array_element _outactors
      (`self.K2_DestroyActor` _array_element))
    (else
      (`self.SpawnShootingTarget`)
      (`self.SpawnShootingTarget`)
      (`self.SpawnShootingTarget`))))

(event `SpawnCharacterTarget`
  (set `self.TempSpawnSuccess` false)
  (for _ (range 31)
    (if (not (`self.TempSpawnSuccess`))
      (bind _outactors (`GameplayStatics.GetAllActorsWithTag` "CharacterSpawnBox"))
      (bind (_origin _boxextent) (`self.GetActorBounds` (`|GetArrayItem` _outactors) false false))
      (set `self.TempRandomPoint` (`KismetMathLibrary.MakeVector` (.x (`KismetMathLibrary.RandomPointInBoundingBox` _origin _boxextent)) (.y (`KismetMathLibrary.RandomPointInBoundingBox` _origin _boxextent)) -368.306314))
      (bind (_outactors_2 _returnvalue) (`KismetSystemLibrary.CapsuleOverlapActors` (`self.TempRandomPoint`) 34.0 88.0 (`|MakeArray` "ObjectTypeQuery3" :!type "EObjectTypeQuery Enum")))
      (if (not _returnvalue)
        (`|SpawnActorFromClass` "/Game/Blueprints/Targets/BP_FPS_EnemyTarget.BP_FPS_EnemyTarget_C" (`KismetMathLibrary.MakeTransform` (`self.TempRandomPoint`) (`self.K2_GetActorRotation`)) "Undefined" "MultiplyWithRoot" null null)
        (set `self.TempSpawnSuccess` true)))))

(event `SpawnShootingTarget`
  (set `self.TempSpawnSuccess` false)
  (for _ (range 101)
    (if (not (`self.TempSpawnSuccess`))
      (bind _outactors (`GameplayStatics.GetAllActorsWithTag` "ShootingTargetSpawnBox"))
      (bind (_origin _boxextent) (`self.GetActorBounds` (`|GetArrayItem` _outactors) false false))
      (set `self.TempRandomPoint` (`KismetMathLibrary.RandomPointInBoundingBox` _origin _boxextent))
      (bind (_outactors_2 _returnvalue) (`KismetSystemLibrary.BoxOverlapActors` (`self.TempRandomPoint`) (18.0 65.0 65.0) (`|MakeArray` "ObjectTypeQuery1" "ObjectTypeQuery2" :!type "EObjectTypeQuery Enum") "/Game/Blueprints/Targets/BP_ShootingTarget.BP_ShootingTarget_C"))
      (if (not _returnvalue)
        (set `self.TempSpawnSuccess` true)
        (`|SpawnActorFromClass` "/Game/Blueprints/Targets/BP_ShootingTarget.BP_ShootingTarget_C" (`KismetMathLibrary.MakeTransform` (`self.TEmpRandomPoint`) (`self.K2_GetActorRotation`)) "Undefined" "OverrideRootScale" null null)))))

(fn `UserConstructionScript`)