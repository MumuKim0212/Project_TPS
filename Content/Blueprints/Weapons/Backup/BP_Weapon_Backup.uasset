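; Weapon actor for the FPS fire range that can be dropped with physics, picked up and fired in single, burst or full-auto mode.
; Trigger events drive timed fire loops that play animations and camera shake, then line trace each bullet.
; Hits damage targets and play hit or elimination markers on the main widget, or click mode-check boxes.
; Niagara tracers and surface-type-mapped impact decals, effects and sounds complete each shot.
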(event Custom|DropTo
  (params (InTrm :type Transform))
  (Transformation|SetActorTransform InTrm)
  (Rendering|SetCastShadow (Variables|Default|GetSkeletalMesh) true)
  (Collision|SetCollisionEnabled (Variables|Default|GetSkeletalMesh) "QueryAndPhysics")
  (Variables|일반|픽업드랍|SetCanPickup true))

(event Custom|Pickup
  (Variables|일반|픽업드랍|SetCanPickup false)
  (Physics|SetSimulatePhysics (Variables|Default|GetSkeletalMesh) false)
  (Collision|SetCollisionEnabled (Variables|Default|GetSkeletalMesh) "NoCollision")
  (Transformation|AttachComponentToComponent (Variables|Default|GetSkeletalMesh) (Variables|Default|GetDefaultSceneRoot) "None" "KeepRelative" "KeepRelative" "KeepRelative" true)
  (Transformation|SetRelativeLocationAndRotation (Variables|Default|GetSkeletalMesh) "0, 0, 0" "0, 0, 0" false false))

(event Custom|FireTimerLoop_FullAuto
  (if (or (== (Variables|공개|Ammo|GetAmmo) 0) (not (Variables|일반|Fire|GetPressedTrigger)))
    (Utilities|Time|ClearandInvalidateTimerbyHandle (Variables|일반|Fire|GetFireTimerHandle))
    (Variables|일반|Fire|SetFiring false)
    (else
      (CallFunction|Fire))))

(event Custom|FireTimerLoop_Burst
  (if (or (== (Variables|일반|Fire|GetFireCount) (Variables|공개|GetBurstFireCount)) (== (Variables|공개|Ammo|GetAmmo) 0))
    (Utilities|Time|ClearandInvalidateTimerbyHandle (Variables|일반|Fire|GetFireTimerHandle))
    (Variables|일반|Fire|SetBurstFiring false)
    (else
      (Variables|일반|Fire|SetBurstFiring true)
      (CallFunction|Fire))))

(event Custom|ShowPickup
  (params (InVisible :type Boolean))
  (Rendering|SetVisibility (Variables|Default|GetWidget) InVisible false))

(event Custom|DisablePickup
  (Variables|일반|픽업드랍|SetCanPickup false)
  (Rendering|SetVisibility (Variables|Default|GetWidget) false false)
  (Rendering|SetCastShadow (Variables|Default|GetSkeletalMesh) false)
  (Physics|SetSimulatePhysics (Variables|Default|GetSkeletalMesh) false)
  (Collision|SetCollisionEnabled (Variables|Default|GetSkeletalMesh) "NoCollision")
  (Transformation|AttachComponentToComponent (Variables|Default|GetSkeletalMesh) (Variables|Default|GetDefaultSceneRoot) "None" "KeepRelative" "KeepRelative" "KeepRelative" true)
  (Transformation|SetRelativeLocationAndRotation (Variables|Default|GetSkeletalMesh) "0, 0, 0" "0, 0, 0" false false))

(event Custom|Drop
  (params (InDir :type Vector))
  (Variables|일반|픽업드랍|SetDropping true)
  (Variables|일반|픽업드랍|SetDropTime 0.0)
  (Rendering|SetCastShadow (Variables|Default|GetSkeletalMesh) true)
  (Collision|SetCollisionEnabled (Variables|Default|GetSkeletalMesh) "QueryAndPhysics")
  (Physics|SetSimulatePhysics (Variables|Default|GetSkeletalMesh) true)
  (Physics|AddImpulse (Variables|Default|GetSkeletalMesh) (* InDir 2.4e+02) "None" true))

(event Custom|StopFire
  (if (Variables|일반|Fire|GetPressedTrigger)
    (Variables|일반|Fire|SetPressedTrigger false)))

(event Custom|PressTriggerEvent
  (params (InFireLoc3 :type Vector) (InFireDirection3 :type Vector))
  (CallFunction|UpdateFireInfo InFireLoc3 InFireDirection3 0.0)
  (Utilities|FlowControl|Sequence
    (:then_0
      (Variables|일반|Fire|SetPressedTrigger true))
    (:then_1
      (Variables|일반|Fire|SetFiring true)
      (switch Utilities|FlowControl|Switch|SwitchonE_FireType (Variables|공개|GetFireType)
        (:NewEnumerator0
          (CallFunction|Fire :!pinned true) ; 단발
          (Utilities|FlowControl|Delay (Variables|공개|GetFireDelay))
          (Variables|일반|Fire|SetFiring false)
          (Variables|일반|Fire|SetFireCount 0))
        (:NewEnumerator1
          (bind _returnvalue (Utilities|Time|SetTimerbyEvent (delegate Custom|FireTimerLoop_Burst) (Variables|공개|GetBurstFireDelay) true :!pinned true)) ; 점사
          (Variables|일반|Fire|SetFireTimerHandle _returnvalue)
          (CallFunction|FireTimerLoopBurst)
          (Utilities|FlowControl|Delay (Variables|공개|GetFireDelay))
          (Variables|일반|Fire|SetFiring false)
          (Variables|일반|Fire|SetFireCount 0))
        (:NewEnumerator2
          (bind _returnvalue_2 (Utilities|Time|SetTimerbyEvent (delegate Custom|FireTimerLoop_FullAuto) (Variables|공개|GetFireDelay) true :!pinned true)) ; 연사
          (Variables|일반|Fire|SetFireTimerHandle _returnvalue_2)
          (CallFunction|FireTimerLoopFullAuto))))))

(event Custom|ReleaseTriggerEvent
  (CallFunction|StopFire))

(event Custom|Fire
  (Utilities|FlowControl|Sequence
    (:then_0
      (Math|Integer|IncrementInt (Variables|일반|Fire|GetFireCount)
        (:%20%20
          (Components|Animation|PlayAnimation (Variables|Default|GetSkeletalMesh) (Variables|공개|Animation|GetWeaponFireAnim) false :!pinned true) ; Play Weapon Animation
          (CallFunction|AddAmmo -1)
          (Camera|PlayWorldCameraShake (Variables|공개|GetFireCamShakeClass) (Transformation|GetActorLocation) 0.0 3.5e+02))))
    (:then_1
      (bind _asbp_fps_pcharacter_p3 (Utilities|Casting|CastToBP_FPS_PCharacterP3 (Actor|GetAttachParentActor)))
      (Default|PlayAnimFire _asbp_fps_pcharacter_p3))
    (:then_2
      (bind _asbp_fps_pcharacter_p3_2 (Utilities|Casting|CastToBP_FPS_PCharacterP3 (Actor|GetAttachParentActor))))
    (:then_3
      (|총쏘기라인충돌체크및데미지처리 :!pinned true) ; 총 쏘기 라인 충돌 체크 및 데미지 처리
    )))

(event EventBeginPlay
  (Utilities|FlowControl|DelayUntilNextTick)
  (bind _foundwidgets (Widget|GetAllWidgetsOfClass "/Game/Blueprints/Widgets/WD_MainP3_FireRange.WD_MainP3_FireRange_C" false))
  (Variables|일반|위젯|SetMainWidget (Utilities|Array|Get(acopy) _foundwidgets)))

(event EventTick
  (params (DeltaSeconds :type Float%20%28single-precision%29))
  (bind _skeletalmesh (Variables|Default|GetSkeletalMesh))
  (Utilities|FlowControl|Sequence
    (:then_0
      (if (Variables|일반|픽업드랍|GetDropping)
        (Variables|일반|픽업드랍|SetDropTime (+ (Variables|일반|픽업드랍|GetDropTime) (Utilities|Time|GetWorldDeltaSeconds)))
        (if (and (> (Variables|일반|픽업드랍|GetDropTime) 0.5) (<= (Math|Vector|VectorLength (Transformation|GetComponentVelocity (Variables|Default|GetSkeletalMesh))) 0.1))
          (Variables|일반|픽업드랍|SetDropping false)
          (Variables|일반|픽업드랍|SetCanPickup true))))
    (:then_1
      (if (Class|SceneComponent|IsAnySimulatingPhysics (Variables|Default|GetSkeletalMesh))
        (Transformation|SetActorLocation (Transformation|GetWorldLocation _skeletalmesh) false false)
        (Transformation|SetActorRotation (Transformation|GetWorldRotation _skeletalmesh))))))

(fn ConstructionScript
  (if (Variables|일반|픽업드랍|GetCanPickup)
    (Rendering|SetCastShadow (Variables|Default|GetSkeletalMesh) true)
    (Collision|SetCollisionEnabled (Variables|Default|GetSkeletalMesh) "QueryOnly")
    (else
      (Rendering|SetCastShadow (Variables|Default|GetSkeletalMesh) false)
      (Collision|SetCollisionEnabled (Variables|Default|GetSkeletalMesh) "NoCollision"))))

(fn AddAmmo
  (params (InAmmo :type Integer))
  (Variables|공개|Ammo|SetAmmo (+ InAmmo (Variables|공개|Ammo|GetAmmo))))

(fn CanFire
  (return (and (> (Variables|공개|Ammo|GetAmmo) 0) (not (Variables|일반|Fire|GetFiring)))))

(fn CanReload
  (switch Utilities|FlowControl|Switch|SwitchonE_FireType (Variables|공개|GetFireType)
    (:NewEnumerator0
      _)
    (:NewEnumerator1
      (return (and (< (Variables|공개|Ammo|GetAmmo) (Variables|공개|Ammo|GetMagazineSize)) (not (Variables|일반|Fire|GetBurstFiring)))))
    (:NewEnumerator2
      _))
  (return (< (Variables|공개|Ammo|GetAmmo) (Variables|공개|Ammo|GetMagazineSize))))

(fn UpdateFireInfo
  (params (InFireLoc :type Vector) (InFireDirection :type Vector) (InSpreadFactor :type Float%20%28double-precision%29))
  (Variables|일반|Temp|SetTempFireLoc InFireLoc)
  (Variables|일반|Temp|SetTempFireDirection InFireDirection)
  (Variables|일반|Temp|SetTempSpreadFactor InSpreadFactor))

(fn CanAutoReload
  (switch Utilities|FlowControl|Switch|SwitchonE_FireType (Variables|공개|GetFireType)
    (:NewEnumerator0
      _)
    (:NewEnumerator1
      _)
    (:NewEnumerator2
      _))
  (return (Math|Boolean|ANDBoolean (CallFunction|CanReload) (not (Variables|일반|Fire|GetFiring)) (== (Variables|공개|Ammo|GetAmmo) 0))))

(fn CanPressTrigger
  (return (not (Variables|일반|Fire|GetFiring))))