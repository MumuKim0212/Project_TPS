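; Firearm actor for an FPS firing range, with pickup/drop states, ammo and reload checks, and single, burst and full-auto fire.
; Timer-driven shots update the owning character's spread, recoil and animation, then line trace from the camera in a random spread cone per bullet.
; Hits damage targets with hit-marker or elimination feedback, or click mode-selection boxes.
; Niagara tracers and surface-type-mapped decals, effects and sounds visualize each shot.
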(event EventBeginPlay
  (Utilities|FlowControl|DelayUntilNextTick)
  (bind _foundwidgets (Widget|GetAllWidgetsOfClass "/Game/Blueprints/Widgets/WD_MainP3_FireRange.WD_MainP3_FireRange_C" false))
  (Variables|일반|위젯|SetMainWidget (Utilities|Array|Get(acopy) _foundwidgets)))

(fn ConstructionScript
  (if (Variables|일반|픽업드랍|GetCanPickup)
    (Rendering|SetCastShadow (Variables|Default|GetSkeletalMesh) true)
    (Collision|SetCollisionEnabled (Variables|Default|GetSkeletalMesh) "QueryOnly")
    (else
      (Rendering|SetCastShadow (Variables|Default|GetSkeletalMesh) false)
      (Collision|SetCollisionEnabled (Variables|Default|GetSkeletalMesh) "NoCollision"))))

(fn AddAmmo
  (params (InAmmo :type Integer))
  (Variables|공개|Ammo|SetAmmo (+ InAmmo (Variables|공개|Ammo|GetAmmo))))

(fn CanFire
  (return (and (> (Variables|공개|Ammo|GetAmmo) 0) (not (Variables|일반|Fire|GetFiring)))))

(fn CanReload
  (switch Utilities|FlowControl|Switch|SwitchonE_FireType (Variables|공개|GetFireType)
    (:NewEnumerator0
      _)
    (:NewEnumerator1
      (return (and (< (Variables|공개|Ammo|GetAmmo) (Variables|공개|Ammo|GetMagazineSize)) (not (Variables|일반|Fire|GetBurstFiring)))))
    (:NewEnumerator2
      _))
  (return (< (Variables|공개|Ammo|GetAmmo) (Variables|공개|Ammo|GetMagazineSize))))

(fn CanAutoReload
  (switch Utilities|FlowControl|Switch|SwitchonE_FireType (Variables|공개|GetFireType)
    (:NewEnumerator0
      _)
    (:NewEnumerator1
      _)
    (:NewEnumerator2
      _))
  (return (Math|Boolean|ANDBoolean (CallFunction|CanReload) (not (Variables|일반|Fire|GetFiring)) (== (Variables|공개|Ammo|GetAmmo) 0))))

(event Custom|DropTo
  (params (InTrm :type Transform))
  (Transformation|SetActorTransform InTrm)
  (Rendering|SetCastShadow (Variables|Default|GetSkeletalMesh) true)
  (Collision|SetCollisionEnabled (Variables|Default|GetSkeletalMesh) "QueryAndPhysics")
  (Variables|일반|픽업드랍|SetCanPickup true))

(event Custom|Pickup
  (Variables|일반|픽업드랍|SetCanPickup false)
  (Physics|SetSimulatePhysics (Variables|Default|GetSkeletalMesh) false)
  (Collision|SetCollisionEnabled (Variables|Default|GetSkeletalMesh) "NoCollision")
  (Transformation|AttachComponentToComponent (Variables|Default|GetSkeletalMesh) (Variables|Default|GetDefaultSceneRoot) "None" "KeepRelative" "KeepRelative" "KeepRelative" true)
  (Transformation|SetRelativeLocationAndRotation (Variables|Default|GetSkeletalMesh) "0, 0, 0" "0, 0, 0" false false))

(event Custom|ShowPickup
  (params (InVisible :type Boolean))
  (Rendering|SetVisibility (Variables|Default|GetWidget) InVisible false))

(event Custom|DisablePickup
  (Variables|일반|픽업드랍|SetCanPickup false)
  (Rendering|SetVisibility (Variables|Default|GetWidget) false false)
  (Rendering|SetCastShadow (Variables|Default|GetSkeletalMesh) false)
  (Physics|SetSimulatePhysics (Variables|Default|GetSkeletalMesh) false)
  (Collision|SetCollisionEnabled (Variables|Default|GetSkeletalMesh) "NoCollision")
  (Transformation|AttachComponentToComponent (Variables|Default|GetSkeletalMesh) (Variables|Default|GetDefaultSceneRoot) "None" "KeepRelative" "KeepRelative" "KeepRelative" true)
  (Transformation|SetRelativeLocationAndRotation (Variables|Default|GetSkeletalMesh) "0, 0, 0" "0, 0, 0" false false))

(event Custom|FireTimerLoop_FullAuto
  (if (or (== (Variables|공개|Ammo|GetAmmo) 0) (not (Variables|일반|Fire|GetPullTrigger))) ; 탄약이 없거나 방아쇠를 당기지 않았으면 총 쏘기를 멈춤
    (Utilities|Time|ClearandInvalidateTimerbyHandle (Variables|일반|Fire|GetFireTimerHandle))
    (Variables|일반|Fire|SetFiring false)
    (else
      (CallFunction|Fire))))

(event Custom|FireTimerLoop_Burst
  (if (or (== (Variables|일반|Fire|GetFireCount) (Variables|공개|GetBurstFireCount)) (== (Variables|공개|Ammo|GetAmmo) 0)) ; BurstCount 만큼 쐈거나 탄약이 없으면 총쏘기를 멈춤
    (Utilities|Time|ClearandInvalidateTimerbyHandle (Variables|일반|Fire|GetFireTimerHandle))
    (Variables|일반|Fire|SetBurstFiring false)
    (else
      (Variables|일반|Fire|SetBurstFiring true)
      (CallFunction|Fire))))

(event Custom|PullTriggerEvent
  (Utilities|FlowControl|Sequence
    (:then_0
      (Variables|일반|Fire|SetPullTrigger true))
    (:then_1
      (Variables|일반|Fire|SetFiring true)
      (switch Utilities|FlowControl|Switch|SwitchonE_FireType (Variables|공개|GetFireType)
        (:NewEnumerator0
          (CallFunction|Fire :!pinned true) ; 단발(Single)
          (Utilities|FlowControl|Delay (Variables|공개|GetFireDelay))
          (Variables|일반|Fire|SetFiring false)
          (Variables|일반|Fire|SetFireCount 0))
        (:NewEnumerator1
          (bind _returnvalue (Utilities|Time|SetTimerbyEvent (delegate Custom|FireTimerLoop_Burst) (Variables|공개|GetBurstFireDelay) true :!pinned true)) ; 점사(Burst)
          (Variables|일반|Fire|SetFireTimerHandle _returnvalue)
          (CallFunction|FireTimerLoopBurst)
          (Utilities|FlowControl|Delay (Variables|공개|GetFireDelay))
          (Variables|일반|Fire|SetFiring false)
          (Variables|일반|Fire|SetFireCount 0))
        (:NewEnumerator2
          (bind _returnvalue_2 (Utilities|Time|SetTimerbyEvent (delegate Custom|FireTimerLoop_FullAuto) (Variables|공개|GetFireDelay) true :!pinned true)) ; 연사(Full Auto)
          (Variables|일반|Fire|SetFireTimerHandle _returnvalue_2)
          (CallFunction|FireTimerLoopFullAuto))))))

(event Custom|ReleaseTriggerEvent
  (if (Variables|일반|Fire|GetPullTrigger)
    (Variables|일반|Fire|SetPullTrigger false)))

(event Custom|Fire
  (Utilities|FlowControl|Sequence
    (:then_0
      (bind _asbp_fps_pcharacter_p3 (Utilities|Casting|CastToBP_FPS_PCharacterP3 (Actor|GetAttachParentActor))) ; 플레이어 캐릭터 변수에 저장
      (Variables|일반|SetOwnerCharacter _asbp_fps_pcharacter_p3))
    (:then_1
      (Math|Integer|IncrementInt (Variables|일반|Fire|GetFireCount) ; 총쏜 카운트 증가
        (:%20%20
          (CallFunction|AddAmmo -1) ; 탄약 1감소
          (Default|AddFireSpread (Variables|일반|GetOwnerCharacter)) ; 총 쏠 때 퍼짐을 높임(정확도 를 낮춤)
          (Default|AddFireRecoil (Variables|일반|GetOwnerCharacter)) ; 총기 반동을 추가
          (Default|PlayAnimFire (Variables|일반|GetOwnerCharacter)) ; 캐릭터 총 쏘는 애니메이션 플레이
          (Components|Animation|PlayAnimation (Variables|Default|GetSkeletalMesh) (Variables|공개|Animation|GetWeaponFireAnim) false :!pinned true) ; 무기 총 쏘는 애니메이션 플레이
          (Camera|PlayWorldCameraShake (Variables|공개|GetFireCamShakeClass) (Transformation|GetActorLocation) 0.0 3.5e+02) ; 카메라 진동
        )))
    (:then_2
      (for _index (range 0 (- (Variables|공개|GetFireBulletCount) 1)) ; 총 쏠때 나가는 총알 갯수 만큼 반복
        (Utilities|FlowControl|Sequence
          (:then_0
            (|LinetraceAndSaveHitInfo :!pinned true) ; Linetrace and Save Hit Info(라인 트레이스 충돌 체크 및 충돌 정보 저장)
          )
          (:then_1
            (|타겟데미지적용및체크박스클릭 :!pinned true) ; Target Apply Damage(타겟 데미지 적용 및 체크 박스 클릭)
          )
          (:then_2
            (|FireTracerEffectsGraph :!pinned true) ; Fire Tracer Effects Graph(총 쏘는 트레이서 이펙트)
          )
          (:then_3
            (|ImpactEffectsGraph :!pinned true) ; Impact Effects Graph (총에 맞은 부분 이펙트)
          ))))))