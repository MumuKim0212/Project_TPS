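; Blueprint function library with helpers that set material parameters across a whole actor.
; One function sets a scalar and the other a vector, each taking a target actor, parameter name and value.
; Both gather every MeshComponent on the actor and apply the value to all materials on each, covering static and skeletal meshes alike.
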(fn `SetScalarParameterValueOnAllMeshComponents`
  (params (InTargetActor :type "Actor Object Reference") (InParamName :type Name) (InParamValue :type "Float (double-precision)"))
  (for _array_element (`Actor.K2_GetComponentsByClass` (`local.InTargetActor`) "/Script/Engine.MeshComponent")
    (`MeshComponent.SetScalarParameterValueOnMaterials` _array_element (`local.InParamName`) (`local.InParamValue`))))

(fn `SetVectorParameterValueOnAllMeshComponents`
  (params (InTargetActor :type "Actor Object Reference") (InParamName :type Name) (InParamValue :type "Vector Structure"))
  (for _array_element (`Actor.K2_GetComponentsByClass` (`local.InTargetActor`) "/Script/Engine.MeshComponent")
    (`MeshComponent.SetVectorParameterValueOnMaterials` _array_element (`local.InParamName`) (`local.InParamValue`))))